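; Snowman controller actor that spawns a group of snowmen and manages their shared target and updates.
; SpawnSnowmen lays them out in a grid from its own transform using a per-row count and spacing, printing each position.
; SpawnSnowman stores each in an array and hands it the controller and target.
; CallSnowmanUpdate passes elapsed time and target to every snowman, then resets the timer; the event graph is empty.
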(event EventBeginPlay)

(event Collision|EventActorBeginOverlap
  (params (OtherActor :type Actor%20Object%20Reference)))

(event EventTick
  (params (DeltaSeconds :type Float%20%28single-precision%29)))

(fn ConstructionScript)

(fn SpawnSnowman
  (params (TransformOfSpawn :type Transform))
  (bind _returnvalue (Game|SpawnActorfromClass "/Game/Blueprints/Snowman.Snowman_C" TransformOfSpawn "AlwaysSpawn" self 0))
  (Utilities|Array|Add (Variables|Default|Get_mSnowmanArray) _returnvalue)
  (Variables|/Game/Blueprints/Snowman.Snowman_C|Set_mController _returnvalue self)
  (Variables|/Game/Blueprints/Snowman.Snowman_C|SetTarget _returnvalue (Variables|Default|GetTarget)))

(fn SpawnSnowmen
  (params (NumberToSpawn :type Integer))
  (bind _returnvalue (Transformation|GetActorTransform))
  (bind _snowmenperrow (Variables|Default|GetSnowmenPerRow))
  (bind _differenceinpositions (Variables|Default|GetDifferenceInPositions))
  (LocalVariables|SetCounter 0)
  (while (< (LocalVariables|GetCounter) NumberToSpawn)
    (Development|PrintString (Utilities|String|ToString(Vector) (Math|Vector|MakeVector (+ (* (.x _differenceinpositions) (Math|Conversions|ToFloat(Integer) (Math|Integer|%(Integer) (LocalVariables|GetCounter) _snowmenperrow))) (.x (.location _returnvalue))) (+ (* (.y _differenceinpositions) (Math|Conversions|ToFloat(Integer) (/ (LocalVariables|GetCounter) _snowmenperrow))) (.y (.location _returnvalue))) (.z (.location _returnvalue)))))
    (CallFunction|SpawnSnowman (Math|Transform|MakeTransform (Math|Vector|MakeVector (+ (* (.x _differenceinpositions) (Math|Conversions|ToFloat(Integer) (Math|Integer|%(Integer) (LocalVariables|GetCounter) _snowmenperrow))) (.x (.location _returnvalue))) (+ (* (.y _differenceinpositions) (Math|Conversions|ToFloat(Integer) (/ (LocalVariables|GetCounter) _snowmenperrow))) (.y (.location _returnvalue))) (.z (.location _returnvalue))) (.rotation _returnvalue) (.scale _returnvalue)))
    (Math|Integer|IncrementInt (LocalVariables|GetCounter)))
  (Variables|Default|SetnumberOfSnowmenHeld (+ NumberToSpawn (Variables|Default|GetnumberOfSnowmenHeld))))

(fn CallSnowmanUpdate
  (for _array_element (Variables|Default|Get_mSnowmanArray)
    (Default|Update _array_element (Variables|Default|GettimeSinceLastUpdate) (Variables|Default|GetTarget self)))
  (Variables|Default|SettimeSinceLastUpdate 0.0))