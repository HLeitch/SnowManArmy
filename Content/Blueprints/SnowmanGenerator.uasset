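; Spawner actor that creates the game's snowmen and drives their updates toward the player's position.
; On BeginPlay it spawns a row of SnowmanController actors offset along X, each spawning an equal share of the snowmen.
; Tick adds delta time to every controller but updates only one per frame in round-robin, passing it the player's location, so the update cost is spread across frames.
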(event EventBeginPlay
  (Variables|Default|SetPlayer (Variables|Default|GetPlayer))
  (Variables|Default|SetSnowmen%20Per%20Group (/ (Variables|Default|GetNumberofSnowmen) (Variables|Default|GetNumberOfGroups)))
  (CallFunction|CreateSnowmanControllers))

(event Collision|EventActorBeginOverlap
  (params (OtherActor :type Actor%20Object%20Reference)))

(event EventTick
  (params (DeltaSeconds :type Float%20%28single-precision%29))
  (bind _snowmancontrollers (Variables|Default|GetsnowmanControllers))
  (Variables|Default|SetDeltaTime DeltaSeconds)
  ;[1 1 1] Update the time step in each Snowman Controller
  (for _array_element _snowmancontrollers
    (Variables|/Game/Blueprints/SnowmanController.SnowmanController_C|SettimeSinceLastUpdate _array_element (+ (Variables|Default|GetDeltaTime) (Variables|/Game/Blueprints/SnowmanController.SnowmanController_C|GettimeSinceLastUpdate _array_element))))
  (bind _targetposition (CallFunction|GetPlayerPosition))
  ;[1 1 1] Seperate update into a number of groups.
  (Variables|/Game/Blueprints/SnowmanController.SnowmanController_C|SetTarget (Utilities|Array|Get(acopy) _snowmancontrollers (Variables|Default|GetindexOfTickGroup)) _targetposition)
  (Default|CallSnowmanUpdate (Utilities|Array|Get(acopy) _snowmancontrollers (Variables|Default|GetindexOfTickGroup)))
  (bind _result (Math|Integer|IncrementInt (Variables|Default|GetindexOfTickGroup))
    (:%20%20
      (if (not (> (Variables|Default|GetNumberOfGroups) _result))
        (Variables|Default|SetindexOfTickGroup 0)))))

(fn ConstructionScript)

(fn CreateSnowmanControllers
  (bind _returnvalue (Transformation|GetActorTransform))
  (for _index (range 0 (- (Variables|Default|GetNumberOfGroups) 1))
    (bind _returnvalue_2 (Game|SpawnActorfromClass "/Game/Blueprints/SnowmanController.SnowmanController_C" (Math|Transform|MakeTransform (Math|Vector|MakeVector (+ (.x (.location _returnvalue)) (* _index (Variables|Default|GetDistanceBetweenSpawners))) (.y (.location _returnvalue)) (.z (.location _returnvalue))) (.rotation _returnvalue) (.scale _returnvalue)) "Undefined" self 0 0))
    (bind _targetposition (CallFunction|GetPlayerPosition))
    (Variables|/Game/Blueprints/SnowmanController.SnowmanController_C|SetTarget _returnvalue_2 _targetposition)
    (Utilities|Array|Add (Variables|Default|GetsnowmanControllers) _returnvalue_2)
    (Default|SpawnSnowmen _returnvalue_2 (Variables|Default|GetSnowmen%20Per%20Group))))

(fn GetPlayerPosition
  (bind _output_get (Variables|Default|SetAttackingTarget (Transformation|GetWorldLocation (Variables|/Script/Engine.Actor|GetRootComponent (Variables|Default|GetPlayer)))))
  (return _output_get))