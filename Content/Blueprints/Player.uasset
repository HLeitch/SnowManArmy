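; Player-controlled snowman that walks, turns and throws snowballs, glowing brighter with each enemy killed.
; Tick runs Movement, which sets the walking flag, offsets the actor along the collider's forward vector without sweep and applies yaw.
; Releasing Space sets the throwing flag, then after a short delay spawns a Snowball launched by impulse.
; EnemyKilled raises emissive strength on a dynamic lava material; ChangeVertexColour only performs a downward debug trace.
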(event Custom|FireSnowball
  (Variables|Default|SetIsThrowing true)
  (GameplayTasks|TaskWaitDelay (Variables|Default|GettaskOwner) 0.5
    (:OnFinish
      (CallFunction|FiringSnowball))))

(event EventBeginPlay
  (bind _returnvalue (Rendering|Material|CreateDynamicMaterialInstance (Variables|Default|GetSnowmanAnimated_WalkingAndThrowing1) 1 "/Game/Materials/LavaMan_Inst.LavaMan_Inst" "None" :!class /Script/Engine.PrimitiveComponent))
  (Variables|Default|SetMyLavaMaterial _returnvalue))

(event Collision|EventActorBeginOverlap
  (params (OtherActor :type Actor%20Object%20Reference)))

(event EventTick
  (params (DeltaSeconds :type Float%20%28single-precision%29))
  (CallFunction|Movement))

(event Input|KeyboardEvents|SpaceBar
  (params (Key :type Key%20Structure :default "None"))
  (:Released
    (CallFunction|FireSnowball)))

(fn ConstructionScript)

(fn Movement
  (bind _returnvalue (Transformation|GetActorRotation))
  (bind _returnvalue_2 (Input|AxisValues|GetMoveForward))
  (if (> _returnvalue_2 0.0)
    (Variables|Default|SetIsWalking true)
    (else
      (Variables|Default|SetIsWalking false)))
  (Transformation|AddActorWorldOffset (* (* (Math|Vector|GetForwardVector (Variables|Default|GetmovementCollider)) _returnvalue_2) (Variables|Default|GetMovementForce)))
  (Transformation|SetActorRotation (Math|Rotator|MakeRotator (.roll _returnvalue) (.pitch _returnvalue) (+ (* (Input|AxisValues|GetMoveRight) (Variables|Default|GetRotationRate)) (.yaw _returnvalue)))))

(fn ChangeVertexColour
  (bind _returnvalue (Transformation|GetActorLocation))
  (Collision|LineTraceByChannel _returnvalue (+ _returnvalue (* (Math|Vector|VectorDown) 3e+02)) "TraceTypeQuery1" false 0 "ForDuration"))

(fn EnemyKilled
  (bind _mylavamaterial (Variables|Default|GetMyLavaMaterial))
  (bind _output_get (Variables|Default|SetGlowValue (+ (Variables|Default|GetGlowValue) (Variables|Default|GetGlowIncreasePerEnemyKilled))))
  (Rendering|Material|GetScalarParameterValue _mylavamaterial "Emissive Strength" :!class /Script/Engine.MaterialInstanceDynamic)
  (Rendering|Material|SetScalarParameterValue _mylavamaterial "Emissive Strength" _output_get :!class /Script/Engine.MaterialInstanceDynamic))

(fn FiringSnowball
  (bind _returnvalue (Transformation|GetActorForwardVector))
  (bind _throwforcex (Variables|Default|GetThrowForceX))
  (bind _returnvalue_2 (* _returnvalue _throwforcex))
  (bind _returnvalue_3 (Game|SpawnActorfromClass "/Game/Blueprints/Snowball.Snowball_C" (Math|Transform|MakeTransform (Math|Transform|TransformLocation (Transformation|GetActorTransform) (Variables|Default|GetSnowballFire)) "0, 0, 0" "1,1,1") "Undefined" self 0))
  (Physics|AddImpulse (Variables|/Game/Blueprints/Snowball.Snowball_C|GetBall _returnvalue_3) (Math|Vector|MakeVector (.x _returnvalue_2) (.y _returnvalue_2) (Variables|Default|GetThrowForceZ)) "None" true)
  (Variables|Default|SetIsThrowing false))