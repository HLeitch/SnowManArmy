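; Snowman enemy that uses boid-style steering to chase a supplied target within range and melts when hit by a snowball.
; Update sums target attraction and distance-scaled avoidance of overlapping snowmen, without clearing earlier directions, to offset its vertex-animated body.
; A snowball hit destroys the hit actor, spawns particles and starts a looping timer that shrinks the snowman.
; Once tiny, it notifies the Player of the kill, destroys itself and leaves MController's array.
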(event Custom|Melting
  (Utilities|Time|SetTimerbyFunctionName self "Melt" 0.02 true)
  (Niagara|SpawnSystematLocation "/Game/Materials/SnowmanBuildingParticles.SnowmanBuildingParticles" (Transformation|GetActorLocation)))

(event EventBeginPlay
  (Variables|Default|SetBoidEffectDistance (Variables|/Script/Engine.SphereComponent|GetSphereRadius (Variables|Default|GetBoidBehaviour)))
  (Components|Tick|SetComponentTickEnabled (Variables|Default|GetBoidBehaviour) true))

(event Collision|EventActorBeginOverlap
  (params (OtherActor :type Actor%20Object%20Reference)))

(event EventTick
  (params (DeltaSeconds :type Float%20%28single-precision%29)))

(event Collision|EventHit
  (params (MyComp :type Primitive%20Component%20Object%20Reference) (Other :type Actor%20Object%20Reference) (OtherComp :type Primitive%20Component%20Object%20Reference) (bSelfMoved :type Boolean) (HitLocation :type Vector :default "0, 0, 0") (HitNormal :type Vector :default "0, 0, 0") (NormalImpulse :type Vector :default "0, 0, 0") (Hit :type Hit%20Result%20Structure%20%28by%20ref%29))
  (if (== (Utilities|GetClass Other) "/Game/Blueprints/Snowball.Snowball_C")
    (Variables|Default|SetisMelting true)
    (CallFunction|SnowballHit Hit)))

(event EventDestroyed
  (Utilities|Array|RemoveItem (Variables|/Game/Blueprints/SnowmanController.SnowmanController_C|Get_mSnowmanArray (Variables|Default|Get_mController)) self))

(fn ConstructionScript)

(fn Update
  (params (timeSinceLast%20Update :type Float%20%28single-precision%29) (TargetPos :type Vector))
  (bind _returnvalue (Transformation|GetActorLocation))
  (bind _returnvalue_2 (Transformation|GetActorLocation))
  (Variables|Default|SetTarget TargetPos)
  (LocalVariables|SetDeltaTime timeSinceLast%20Update)
  (if (< (Math|Vector|Distance(Vector) _returnvalue_2 (Variables|Default|GetTarget)) (Variables|Default|GetMaxDistanceFromTarget))
    (Utilities|Array|Add (LocalVariables|GetDirectionsToTravel) (* (Math|Vector|GetUnitDirection(Vector) _returnvalue_2 (Variables|Default|GetTarget)) (Variables|Default|GetTargetDirectionStrength)))
    (for _array_element (Collision|GetOverlappingActors (Variables|Default|GetBoidBehaviour) "Snowman_C" :!class /Script/Engine.PrimitiveComponent)
      (if (== (Utilities|GetClass _array_element) "Snowman_C")
        (if (!= _array_element self)
          (Utilities|Array|Add (LocalVariables|GetDirectionsToTravel) (* (* (Math|Vector|GetUnitDirection(Vector) _returnvalue (Transformation|GetActorLocation _array_element)) "-1.000000,-1.000000, 0") (* (Variables|Default|GetMaxAvoidingStrength) (/ (Math|Vector|Distance(Vector) (Transformation|GetActorLocation _array_element) _returnvalue) (Variables|Default|GetBoidEffectDistance))))))))
    ;[1 1 1] Output
    (for _array_element_2 (LocalVariables|GetDirectionsToTravel)
      (LocalVariables|SetFinalDirection (+ (LocalVariables|GetFinalDirection) _array_element_2)))
    (Transformation|AddWorldOffset (Variables|Default|GetSnowmanVertAnim_Body) (* (Math|Vector|Normalize (LocalVariables|GetFinalDirection)) (* (Variables|Default|GetMoveSpeed) (LocalVariables|GetDeltaTime))) false false)))

(fn SnowballHit
  (params (HitResult :type Hit%20Result%20Structure))
  (CallFunction|Melting)
  (Actor|DestroyActor (.hitactor HitResult)))

(fn Melt
  (if (Variables|Default|GetisMelting)
    (Transformation|SetActorScale3D (- (Transformation|GetActorScale3D) (* (Variables|Default|GetMeltingRate) (Math|Conversions|ToVector(Float) (Utilities|Time|GetWorldDeltaSeconds)))))
    (if (> 0.05 (.z (Transformation|GetActorScale3D)))
      (Variables|Default|SetisMelting false)
      (bind _returnvalue (Actor|GetActorOfClass "/Game/Blueprints/Player.Player_C"))
      (Default|EnemyKilled _returnvalue)
      (Actor|DestroyActor))))